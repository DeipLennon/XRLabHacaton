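; BPC_LabiribtGenerator builds a labyrinth by scattering BP_LabWall actors at random.
; Its LabGen function spawns a requested count of walls at random X/Y positions within a fixed rectangle at zero height, each randomly yawed 0 or 90 degrees.
; Spawned walls are stored in WallRefs; placement has no grid, overlap or path checks.
; The event graph is empty, so generation depends on an external call.
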(event EventBeginPlay)

(event EventTick
  (params (DeltaSeconds :type Float%20%28single-precision%29)))

(fn LabGen
  (params (Count :type Integer))
  (for _index (range 0 (- Count 1))
    (bind _returnvalue (Game|SpawnActorfromClass "/Game/Blueprints/BP_LabWall.BP_LabWall_C" (Math|Transform|MakeTransform (Math|Vector|MakeVector (Math|Random|RandomFloatinRange -1e+03 1e+03) (Math|Random|RandomFloatinRange -2e+03 2e+03) 0.0) (select (Math|Random|RandomBool) (Math|Rotator|MakeRotator 0.0 0.0 9e+01) (Math|Rotator|MakeRotator 0.0 0.0 0.0)) "1.000000,1.000000,1.000000") "Undefined" 0 0))
    (Utilities|Array|AddUnique (Variables|Default|GetWallRefs) _returnvalue)))